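; Actor component that handles interaction input and shows a 3D prompt on the owner's current interactable.
; On BeginPlay it spawns a hidden BP_InteractionPrompt_3D, hands it the owner's camera component and caches its widget.
; When the interactable changes, it attaches the prompt using the offset and transform that target supplies, or hides it if none is valid.
; IA_Interact sends an interact message to the current interactable.
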(event Input|EnhancedActionEvents|EnhancedInputActionIA_Interact
  (params (ActionValue :type Boolean) (ElapsedSeconds :type Float%20%28double-precision%29) (TriggeredSeconds :type Float%20%28double-precision%29) (InputAction :type Input%20Action%20Object%20Reference :default "/Game/ThirdPerson/Input/Actions/IA_Interact.IA_Interact"))
  (Class|Interactable|Interact(Message) (Variables|Default|GetCurrentInteractable)))

(event EventBeginPlay
  (bind _returnvalue (Components|GetOwner))
  (bind _returnvalue_2 (Game|SpawnActorfromClass "/Game/Blueprints/BP_InteractionPrompt_3D.BP_InteractionPrompt_3D_C" (Math|Transform|MakeTransform (Transformation|GetActorLocation _returnvalue) "0, 0, 0" "1.000000,1.000000,1.000000") "Undefined" "MultiplyWithRoot" 0 0))
  (Actor|SetOwner _returnvalue_2 _returnvalue)
  (Rendering|SetVisibility (Variables|/Game/Blueprints/BP_InteractionPrompt_3D.BP_InteractionPrompt_3D_C|GetWidget _returnvalue_2) false false)
  (Default|SetPlayerCameraManager _returnvalue_2 (Actor|GetComponentbyClass _returnvalue "/Script/Engine.CameraComponent"))
  (Variables|Default|SetWidget (Variables|/Game/Blueprints/BP_InteractionPrompt_3D.BP_InteractionPrompt_3D_C|GetWidget _returnvalue_2)))

(event EventOnInteractableChanged
  (bind _widget (Variables|Default|GetWidget))
  (bind _currentinteractable (Variables|Default|GetCurrentInteractable))
  (if (Utilities|IsValid _currentinteractable)
    (bind _returnvalue (Class|Interactable|GetInteractionPromptOffset(Message) _currentinteractable))
    (Class|InteractionFunctionLibrary|AppendInteractionPrompttoInteractableActor _widget _returnvalue (Transformation|GetActorTransform _currentinteractable))
    (else
      (Class|InteractionFunctionLibrary|HideInteractionPrompt _widget))))