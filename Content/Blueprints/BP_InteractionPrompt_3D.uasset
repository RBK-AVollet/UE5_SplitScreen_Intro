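; BP_InteractionPrompt_3D is a world-space interaction prompt that keeps its widget facing the player's camera.
; Each tick, while the widget is visible and the camera manager is valid, it rotates the widget with a look-at rotation toward that camera manager's location.
; The camera manager is supplied from outside through SetPlayerCameraManager rather than looked up by the prompt itself.
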(event EventBeginPlay)

(event EventTick
  (params (DeltaSeconds :type Float%20%28single-precision%29))
  (if (and (Rendering|IsVisible (Variables|Default|GetWidget)) (Utilities|IsValid (Variables|Default|GetPlayerCamera%20Manager)))
    (Transformation|SetWorldRotation (Variables|Default|GetWidget) (Math|Rotator|FindLookatRotation (Transformation|GetWorldLocation (Variables|Default|GetWidget)) (Transformation|GetWorldLocation (Variables|Default|GetPlayerCamera%20Manager))) false false)))

(fn ConstructionScript)

(fn SetPlayerCameraManager
  (params (Camera :type Camera%20Component%20Object%20Reference))
  (Variables|Default|SetPlayerCamera%20Manager Camera))